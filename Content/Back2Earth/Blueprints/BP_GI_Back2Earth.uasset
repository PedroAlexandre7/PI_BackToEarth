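; Game instance for Back2Earth that centralizes 2D sound playback and per-level background music.
; PlaySound spawns a given sound at a given volume, persisting across level transitions.
; PlayMusic compares the current level name to a cached one and, on change, stops the old track and spawns that level's track, storing it for later stopping.
; Only the Tutorial and Mars tracks set a reduced volume and persistence across transitions.
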(event Custom|Play%20Sound
  (params (Sound :type Sound%20Wave%20Object%20Reference) (VolumeMultiplier :type Float%20%28single-precision%29))
  (Audio|SpawnSound2D Sound VolumeMultiplier 1.0 0.0 0 true))

(event Custom|Play%20Music
  (bind _returnvalue (Game|GetCurrentLevelName true))
  (if (Utilities|Enum|NotEqual(Enum) _returnvalue (Variables|Default|GetcurrentLevel))
    (Variables|Default|SetcurrentLevel _returnvalue)
    (if (Utilities|IsValid (Variables|Components|GetcurrentMusic))
      (Audio|Components|Audio|Stop (Variables|Components|GetcurrentMusic)))
    (switch string (Variables|Default|GetcurrentLevel)
      (:MainMenu
        (bind _returnvalue_2 (Audio|SpawnSound2D "/Game/Back2Earth/Sounds/MainMenuSpaceMusic.MainMenuSpaceMusic" 0.2 1.0 0.0 0 true))
        (Variables|Components|SetcurrentMusic _returnvalue_2))
      (:Tutorial
        (bind _returnvalue_3 (Audio|SpawnSound2D "/Game/Back2Earth/Sounds/TutorialWiiMusic.TutorialWiiMusic" 0.35 1.0 0.0 0 true))
        (Variables|Components|SetcurrentMusic _returnvalue_3))
      (:Callisto
        (bind _returnvalue_4 (Audio|SpawnSound2D "/Game/Back2Earth/Sounds/NOMA_-_Brain_Power__Off-Vocal_.NOMA_-_Brain_Power__Off-Vocal_" 0.5 1.0 0.0 0 true))
        (Variables|Components|SetcurrentMusic _returnvalue_4))
      (:Mars
        (bind _returnvalue_5 (Audio|SpawnSound2D "/Game/Back2Earth/Sounds/MarsMusic.MarsMusic" 0.35 1.0 0.0 0 true))
        (Variables|Components|SetcurrentMusic _returnvalue_5))
      (:Moon
        (bind _returnvalue_6 (Audio|SpawnSound2D "/Game/Back2Earth/Sounds/Moonlight__Instrumental_.Moonlight__Instrumental_" 0.2 1.0 0.0 0 true))
        (Variables|Components|SetcurrentMusic _returnvalue_6))
      (:Earth
        (bind _returnvalue_7 (Audio|SpawnSound2D "/Game/Back2Earth/Sounds/TerraMusic.TerraMusic" 0.2 1.0 0.0 0 true))
        (Variables|Components|SetcurrentMusic _returnvalue_7)))))
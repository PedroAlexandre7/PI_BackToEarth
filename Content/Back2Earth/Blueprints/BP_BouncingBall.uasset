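; BP_BouncingBall is a bouncing projectile that knocks the third-person player character along at a boosted version of its own velocity.
; It samples a bounce limit from a discrete probability distribution on BeginPlay and plays a hit sound on bounces up to that limit, lowering pitch logarithmically.
; Reaching the limit or hitting the character triggers a one-time slowdown that adjusts bounce physics, ignores Pawn collision and shortens the lifespan to despawn it.
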(event OnProjectileBounce(ProjectileMovement)
  (params (ImpactResult :type Hit%20Result%20Structure%20%28by%20ref%29) (ImpactVelocity :type Vector%20%28by%20ref%29 :default "0, 0, 0"))
  (bind _result (Math|Integer|IncrementInt (Variables|Default|Getcurrent_bounces))
    (:%20%20
      (Math|Integer|CompareInt _result (Variables|Default|Getmax_bounces)
        (:>
          (CallFunction|SlowDownandDespawn :!label _label))
        (:==
          (Utilities|FlowControl|Sequence
            (:then_0
              (goto _label))
            (:then_1
              (Audio|SpawnSoundatLocation "/Game/Back2Earth/Sounds/ES_Wall_Hit_Hollow_-_SFX_Producer.ES_Wall_Hit_Hollow_-_SFX_Producer" (Transformation|GetWorldLocation (Variables|Default|GetSphere)) "0, 0, 0" 1.0 (* (- 1.5 (Math|Float|Log (Math|Conversions|ToFloat(Integer) (Variables|Default|Getcurrent_bounces)) 2e+01)) 1.5) 0.0 "/Game/Back2Earth/Sounds/MissileSoundAttenuation.MissileSoundAttenuation" 0 :!label _label_2))))
        (:<
          (goto _label_2))))))

(event OnComponentHit(CollisionSphere)
  (params (HitComponent :type Primitive%20Component%20Object%20Reference) (OtherActor :type Actor%20Object%20Reference) (OtherComp :type Primitive%20Component%20Object%20Reference) (NormalImpulse :type Vector :default "0, 0, 0") (Hit :type Hit%20Result%20Structure%20%28by%20ref%29))
  (bind _asbp_b2e_third_person_character (Utilities|Casting|CastToBP_B2E_ThirdPersonCharacter OtherActor))
  (Character|LaunchCharacter _asbp_b2e_third_person_character (* (Transformation|GetComponentVelocity (Variables|Default|GetCollisionSphere)) 1.2) false false)
  (CallFunction|SlowDownandDespawn))

(event EventBeginPlay
  (Variables|Default|Setmax_bounces (Math|Float|Truncate (Class|ProbabilityMethods|EmpiricalDiscreteProbabilityNumber (Variables|Default|GetdiracDeltaArray))))
  (Actor|SetLifeSpan 9e+01))

(fn ConstructionScript)

(fn SlowDownandDespawn
  (bind _projectilemovement (Variables|Default|GetProjectileMovement))
  (Utilities|FlowControl|DoOnce false
    (:Completed
      (Variables|/Script/Engine.ProjectileMovementComponent|SetBounciness _projectilemovement 0.25)
      (Variables|/Script/Engine.ProjectileMovementComponent|SetProjectileGravityScale _projectilemovement 1.0)
      (Variables|/Script/Engine.ProjectileMovementComponent|SetFriction _projectilemovement 0.5)
      (Actor|SetLifeSpan 3.0)
      (Collision|SetCollisionResponsetoChannel (Variables|Default|GetCollisionSphere) "ECC_Pawn" "ECR_Ignore"))))
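; Laser spinner hazard that rotates around its yaw axis and kills the third-person character when either of its two cones begins overlapping it.
; Rotation speed, in turns per second, comes from a normal-distribution probability helper fed by a mu/sigma array, generated at BeginPlay and on Reroll.
; Tick applies the frame-rate-independent spin, divided by a slowdown multiplier while the slowed flag set by SpeedDown and cleared by SpeedUp is active.
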(event OnComponentBeginOverlap(Cone1)
  (params (OverlappedComponent :type Primitive%20Component%20Object%20Reference) (OtherActor :type Actor%20Object%20Reference) (OtherComp :type Primitive%20Component%20Object%20Reference) (OtherBodyIndex :type Integer) (bFromSweep :type Boolean) (SweepResult :type Hit%20Result%20Structure%20%28by%20ref%29))
  (bind _asbp_b2e_third_person_character (Utilities|Casting|CastToBP_B2E_ThirdPersonCharacter OtherActor))
  (Default|Death _asbp_b2e_third_person_character))

(event OnComponentBeginOverlap(Cone2)
  (params (OverlappedComponent :type Primitive%20Component%20Object%20Reference) (OtherActor :type Actor%20Object%20Reference) (OtherComp :type Primitive%20Component%20Object%20Reference) (OtherBodyIndex :type Integer) (bFromSweep :type Boolean) (SweepResult :type Hit%20Result%20Structure%20%28by%20ref%29))
  (bind _asbp_b2e_third_person_character (Utilities|Casting|CastToBP_B2E_ThirdPersonCharacter OtherActor))
  (Default|Death _asbp_b2e_third_person_character))

(event Custom|Reroll
  (CallFunction|GenerateRotationSpeed))

(event EventBeginPlay
  (CallFunction|GenerateRotationSpeed))

(event EventTick
  (params (DeltaSeconds :type Float%20%28single-precision%29))
  (bind _currentrotationspeed (Variables|Default|GetcurrentRotationSpeed))
  (bind _returnvalue (* DeltaSeconds _currentrotationspeed 3.6e+02))
  (if (Variables|Default|GetisSlowed)
    (Transformation|AddActorLocalRotation (Math|Rotator|MakeRotator 0.0 0.0 (/ _returnvalue (Variables|Default|GetslowdownMultiplier))) false false)
    (else
      (Transformation|AddActorLocalRotation (Math|Rotator|MakeRotator 0.0 0.0 _returnvalue) false false))))

(fn ConstructionScript)

(fn GenerateRotationSpeed
  (Variables|Default|SetcurrentRotationSpeed (Class|ProbabilityMethods|NormalMultipleProbabilityNumber (Variables|Default|GetMiuSigmaArray))))

(fn SpeedDown
  (if (not (Variables|Default|GetisSlowed))
    (Variables|Default|SetisSlowed true)))

(fn SpeedUp
  (Variables|Default|SetisSlowed false))
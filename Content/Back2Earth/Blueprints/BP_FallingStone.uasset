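; BP_FallingStone is a stone that drops when a BP_B2E_ThirdPersonCharacter enters its box, unless MakeReal has marked it real.
; Falling enables physics, makes the surface unwalkable and destroys the actor after a short lifespan.
; BeginPlay picks the cube's material through a discrete probability function.
; The ShakeOccasionally event drives a pitch-wobble timeline, randomly forward or reversed, repeating after exponentially distributed delays.
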(event OnComponentBeginOverlap(Box)
  (params (OverlappedComponent :type Primitive%20Component%20Object%20Reference) (OtherActor :type Actor%20Object%20Reference) (OtherComp :type Primitive%20Component%20Object%20Reference) (OtherBodyIndex :type Integer) (bFromSweep :type Boolean) (SweepResult :type Hit%20Result%20Structure%20%28by%20ref%29))
  (Utilities|Casting|CastToBP_B2E_ThirdPersonCharacter OtherActor)
  (CallFunction|Fall))

(event Custom|ShakeOccasionally
  (bind _defaultsceneroot (Variables|Default|GetDefaultSceneRoot))
  (bind _returnvalue (Transformation|GetWorldRotation _defaultsceneroot))
  (if (Math|Random|RandomBool) :!label _label
    (bind _rotationy (Timeline|Shake PlayFromStart)
      (:Update
        (Transformation|SetWorldRotation _defaultsceneroot (Math|Rotator|MakeRotator (.roll _returnvalue) (* _rotationy (Variables|Default|GetShakeMultiplier)) (.yaw _returnvalue)) false false))
      (:Finished
        (Utilities|FlowControl|Delay (Class|ProbabilityMethods|ExponentialProbabilityNumber (Variables|Default|GetMinimumShakeInterval) (Variables|Default|GetExponentialShakeInterval)))
        (goto _label)))
    (else
      (Timeline|Shake ReverseFromEnd))))

(event EventBeginPlay
  (Rendering|Material|SetMaterial (Variables|Default|GetCube) 0 (Utilities|Array|Get(acopy) (Variables|Default|GetPossibleMaterials) (Math|Float|Truncate (Class|ProbabilityMethods|EmpiricalDiscreteProbabilityNumber (Variables|Default|GetDiracDeltaProbabilities))))))

(fn ConstructionScript)

(fn MakeReal
  (Variables|Default|SetIsReal true))

(fn Fall
  (if (not (Variables|Default|GetIsReal))
    (Physics|SetSimulatePhysics (Variables|Default|GetCube) true)
    (Class|PrimitiveComponent|SetWalkableSlopeOverride (Variables|Default|GetCube) (Utilities|Struct|MakeWalkableSlopeOverride "WalkableSlope_Unwalkable" 0.0))
    (Actor|SetLifeSpan 5.0)))
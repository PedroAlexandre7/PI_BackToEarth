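; BP_ArrowLauncher is a trap-style launcher that fires volleys of BP_Arrow actors from MissileSpawnArrow after each FireInterval delay.
; Each volley rolls a binomially distributed arrow count between min and max, then fans the arrows randomly or evenly across Spread, in pitch or yaw.
; A non-empty volley plays an attenuated sound and re-arms the delay, so the loop ends permanently once Active is false or the count is zero.
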(event EventBeginPlay
  (Utilities|FlowControl|Delay (Variables|Default|Getfire_interval) :!label _label)
  (Variables|Default|Setcurrent_number_projectiles (Class|ProbabilityMethods|BinomialProbabilityNumberMinMax (Variables|Default|Getmin_projectiles) (Variables|Default|Getmax_projectiles) (Variables|Default|Getbinomial_probability)))
  (if (Variables|Default|GetActive)
    (if (Variables|Default|Getrandom_spread)
      (CallFunction|SpawnProjectileConeRandomSpread)
      (else
        (CallFunction|SpawnProjectileConeDistributedSpread)))
    (Math|Integer|CompareInt (Variables|Default|Getcurrent_number_projectiles)
      (:>
        (Audio|SpawnSoundatLocation "/Game/Back2Earth/Sounds/Arrow_Sound_Effect__online-audio-converter_com_.Arrow_Sound_Effect__online-audio-converter_com_" (Transformation|GetWorldLocation (Variables|Default|GetDefaultSceneRoot)) "0, 0, 0" 0.4 0.8 0.0 "/Game/Back2Earth/Sounds/MissileSoundAttenuation.MissileSoundAttenuation" 0)
        (goto _label))
      (:==))))

(fn ConstructionScript)

(fn SpawnProjectileConeDistributedSpread
  (bind _current_number_projectiles (Variables|Default|Getcurrent_number_projectiles))
  (bind _spread (Variables|Default|Getspread))
  (bind _missilespawnarrow (Variables|Default|GetMissileSpawnArrow))
  (bind _missilespawnarrow_2 (Variables|Default|GetMissileSpawnArrow))
  (bind _returnvalue (Transformation|GetWorldTransform _missilespawnarrow_2))
  (bind _returnvalue_2 (Transformation|GetWorldTransform _missilespawnarrow))
  (bind _returnvalue_3 (- _current_number_projectiles 1))
  (bind _returnvalue_4 (/ _spread -2.0))
  (Math|Integer|CompareInt _current_number_projectiles 1
    (:>
      (for _index (range 0 _returnvalue_3) :!label _label
        (if (Variables|Default|Getvertical_spread)
          (Game|SpawnActorfromClass "/Game/Back2Earth/Blueprints/BP_Arrow.BP_Arrow_C" (Math|Transform|MakeTransform (.location _returnvalue_2) (Math|Rotator|MakeRotator (.roll (.rotation _returnvalue_2)) (+ (.pitch (.rotation _returnvalue_2)) _returnvalue_4 (* _index (/ _spread (Math|Conversions|ToFloat(Integer) _returnvalue_3)))) (.yaw (.rotation _returnvalue_2))) "1.000000,1.000000,1.000000") "AlwaysSpawn" 0 0)
          (else
            (Game|SpawnActorfromClass "/Game/Back2Earth/Blueprints/BP_Arrow.BP_Arrow_C" (Math|Transform|MakeTransform (.location _returnvalue) (Math|Rotator|MakeRotator (.roll (.rotation _returnvalue)) (.pitch (.rotation _returnvalue)) (+ (.yaw (.rotation _returnvalue)) _returnvalue_4 (* _index (/ _spread (Math|Conversions|ToFloat(Integer) _returnvalue_3))))) "1.000000,1.000000,1.000000") "AlwaysSpawn" 0 0)))))
    (:==
      (Game|SpawnActorfromClass "/Game/Back2Earth/Blueprints/BP_Arrow.BP_Arrow_C" (Transformation|GetWorldTransform _missilespawnarrow) "AlwaysSpawn" 0 0))
    (:<
      (goto _label))))

(fn SpawnProjectileConeRandomSpread
  (bind _missilespawnarrow (Variables|Default|GetMissileSpawnArrow))
  (bind _spread (Variables|Default|Getspread))
  (bind _missilespawnarrow_2 (Variables|Default|GetMissileSpawnArrow))
  (bind _returnvalue (Transformation|GetWorldTransform _missilespawnarrow))
  (bind _returnvalue_2 (Transformation|GetWorldTransform _missilespawnarrow_2))
  (bind _returnvalue_3 (Class|ProbabilityMethods|UniformProbabilityNumber 0.0 _spread))
  (bind _returnvalue_4 (/ _spread -2.0))
  (for _index (range 0 (- (Variables|Default|Getcurrent_number_projectiles) 1))
    (if (Variables|Default|Getvertical_spread)
      (Game|SpawnActorfromClass "/Game/Back2Earth/Blueprints/BP_Arrow.BP_Arrow_C" (Math|Transform|MakeTransform (.location _returnvalue_2) (Math|Rotator|MakeRotator (.roll (.rotation _returnvalue_2)) (+ (.pitch (.rotation _returnvalue_2)) _returnvalue_4 _returnvalue_3) (.yaw (.rotation _returnvalue_2))) "1.000000,1.000000,1.000000") "AlwaysSpawn" 0 0)
      (else
        (Game|SpawnActorfromClass "/Game/Back2Earth/Blueprints/BP_Arrow.BP_Arrow_C" (Math|Transform|MakeTransform (.location _returnvalue) (Math|Rotator|MakeRotator (.roll (.rotation _returnvalue)) (.pitch (.rotation _returnvalue)) (+ _returnvalue_4 _returnvalue_3 (.yaw (.rotation _returnvalue)))) "1.000000,1.000000,1.000000") "AlwaysSpawn" 0 0)))))
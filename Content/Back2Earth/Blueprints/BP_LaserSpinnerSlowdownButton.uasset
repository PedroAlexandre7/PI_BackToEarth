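; A floor-trigger button that temporarily slows linked laser spinners when the player character overlaps it.
; On overlap, if not on cooldown, it plays click and slowdown sounds and calls SpeedDown on every spinner in its LaserSpinners array.
; After about ten seconds it plays a speed-up sound, restores the spinners and clears the cooldown, which blocks re-triggering meanwhile.
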(event OnComponentBeginOverlap(Trigger)
  (params (OverlappedComponent :type Primitive%20Component%20Object%20Reference) (OtherActor :type Actor%20Object%20Reference) (OtherComp :type Primitive%20Component%20Object%20Reference) (OtherBodyIndex :type Integer) (bFromSweep :type Boolean) (SweepResult :type Hit%20Result%20Structure%20%28by%20ref%29))
  (if (not (Variables|Default|GetonCooldown))
    (Utilities|Casting|CastToBP_B2E_ThirdPersonCharacter OtherActor)
    (CallFunction|SpinnersSpeedDown)
    (Utilities|FlowControl|RetriggerableDelay 9.9)
    (if (Variables|Default|GetonCooldown)
      (Audio|PlaySound2D "/Game/Back2Earth/Sounds/SpeedUpSound.SpeedUpSound" 2.0 1.0 0.0 0 0)
      (Utilities|FlowControl|Delay 0.1)
      (CallFunction|SpinnersSpeedUp))))

(fn ConstructionScript)

(fn SpinnersSpeedDown
  (Variables|Default|SetonCooldown true)
  (Audio|PlaySound2D "/Engine/VREditor/Sounds/UI/Click_on_Button_Cue.Click_on_Button_Cue" 1.0 1.0 0.0 0 0)
  (Audio|PlaySound2D "/Game/Back2Earth/Sounds/SlowDownSound.SlowDownSound" 2.0 1.0 0.1 "/Game/Back2Earth/Sounds/SingleSoundConcurrency.SingleSoundConcurrency" 0)
  (for _array_element (Variables|Default|GetlaserSpinners)
    (Default|SpeedDown _array_element)))

(fn SpinnersSpeedUp
  (for _array_element (Variables|Default|GetlaserSpinners)
    (Default|SpeedUp _array_element))
  (Variables|Default|SetonCooldown false))
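; BP_SlidingRockSpawner endlessly spawns sliding rocks and launches them along its forward vector.
; From BeginPlay, a Delay loop spawns BP_SlidingRock at a uniform random world-Y offset bounded by root scale, then applies a velocity-change impulse to its boulder.
; Rock scale follows a Rayleigh distribution and spawn intervals an exponential one.
; GetRockParametersworking duplicates the location and scale math but is not called by the event graph.
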(event EventBeginPlay
  (bind _defaultsceneroot (Variables|Default|GetDefaultSceneRoot))
  (bind _returnvalue (Transformation|GetWorldLocation _defaultsceneroot))
  (bind _returnvalue_2 (Transformation|GetWorldScale _defaultsceneroot))
  (bind _returnvalue_3 (Game|SpawnActorfromClass "/Game/Back2Earth/Blueprints/Boulders/BP_SlidingRock.BP_SlidingRock_C" (Math|Transform|MakeTransform (Math|Vector|MakeVector (.x _returnvalue) (+ (.y _returnvalue) (Class|ProbabilityMethods|UniformProbabilityNumber (* (.y _returnvalue_2) -1.0) (.y _returnvalue_2))) (.z _returnvalue)) "0, 0, 0" (Math|Conversions|ToVector(Float) (* (Variables|Default|Getrock_size) (Class|ProbabilityMethods|RayleighProbabilityNumber 1.0 2.0)))) "AdjustIfPossibleButAlwaysSpawn" 0 0 :!label _label))
  (Physics|AddImpulse (Variables|/Game/Back2Earth/Blueprints/Boulders/BP_SlidingRock.BP_SlidingRock_C|GetSandstone%20Boulder _returnvalue_3) (* (Math|Vector|GetForwardVector (Variables|Default|GetDefaultSceneRoot)) 3e+03) "None" true)
  (Utilities|FlowControl|Delay (Class|ProbabilityMethods|ExponentialProbabilityNumber (Variables|Default|Getminimum_spawn_interval) (Variables|Default|Getexponential_spawn_interval)))
  (goto _label))

(fn ConstructionScript)

(fn GetRockParameters,working?
  (bind _defaultsceneroot (Variables|Default|GetDefaultSceneRoot))
  (bind _returnvalue (Transformation|GetWorldLocation _defaultsceneroot))
  (bind _returnvalue_2 (Transformation|GetWorldScale _defaultsceneroot))
  (return (Math|Vector|MakeVector (.x _returnvalue) (+ (Class|ProbabilityMethods|UniformProbabilityNumber (* (.y _returnvalue_2) -1.0) (.y _returnvalue_2)) (.y _returnvalue)) (.z _returnvalue)) (Math|Conversions|ToVector(Float) (* (Variables|Default|Getrock_size) (Class|ProbabilityMethods|RayleighProbabilityNumber 1.0 2.0))) 0.0 0.0 0.0))
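; Meteor debris spawner that drops a randomized rock each time a living third-person player character enters its trigger.
; An empirical discrete distribution picks the debris class, a uniform one offsets it along world Y within a scale-based width, and a Rayleigh one sizes it.
; The rock spawns above the actor and receives a velocity-change impulse.
; With Despawns set, height and vertical impulse switch to alternate values and the rock is marked to despawn.
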(event OnComponentBeginOverlap(Trigger)
  (params (OverlappedComponent :type Primitive%20Component%20Object%20Reference) (OtherActor :type Actor%20Object%20Reference) (OtherComp :type Primitive%20Component%20Object%20Reference) (OtherBodyIndex :type Integer) (bFromSweep :type Boolean) (SweepResult :type Hit%20Result%20Structure%20%28by%20ref%29))
  (bind (_location _scale) (CallFunction|GetRockParameters))
  (bind _asbp_b2e_third_person_character (Utilities|Casting|CastToBP_B2E_ThirdPersonCharacter OtherActor))
  (if (Variables|/Game/Back2Earth/Blueprints/BP_B2E_ThirdPersonCharacter.BP_B2E_ThirdPersonCharacter_C|GetIsAlive _asbp_b2e_third_person_character)
    (bind _asbp_meteor_debris (Utilities|Casting|CastToBP_MeteorDebrisClass (Utilities|Array|Get(acopy) (Variables|Default|GetMeteorDebrisTypes) (Math|Float|Truncate (Class|ProbabilityMethods|EmpiricalDiscreteProbabilityNumber (Variables|Default|GetDiracDeltaArray))))))
    (bind _returnvalue (Game|SpawnActorfromClass _asbp_meteor_debris (Math|Transform|MakeTransform _location "0, 0, 0" _scale) "AlwaysSpawn" 0 0))
    (if (Variables|Despawns|GetDespawns)
      (Default|SettoDespawn _returnvalue))
    (Physics|AddImpulse (Variables|/Game/Back2Earth/Blueprints/Boulders/BP_MeteorDebris.BP_MeteorDebris_C|GetSandstone%20Boulder _returnvalue) (Variables|Default|GetImpulse) "None" true)))

(event EventBeginPlay
  (if (Variables|Despawns|GetDespawns)
    (Variables|Default|SetSpawn%20Height (Variables|Despawns|GetHeightIfDespawns))
    (Variables|Default|SetImpulse (Math|Vector|MakeVector 0.0 0.0 (Variables|Despawns|GetImpulseIfDespawns)))))

(fn ConstructionScript)

(fn GetRockParameters
  (bind _defaultsceneroot (Variables|Default|GetDefaultSceneRoot))
  (bind _returnvalue (Transformation|GetWorldLocation _defaultsceneroot))
  (bind _returnvalue_2 (Transformation|GetWorldScale _defaultsceneroot))
  (bind _returnvalue_3 (* (.x _returnvalue_2) 32.0))
  (return (Math|Vector|MakeVector (.x _returnvalue) (+ (Class|ProbabilityMethods|UniformProbabilityNumber (* _returnvalue_3 -1.0) _returnvalue_3) (.y _returnvalue)) (+ (.z _returnvalue) (Variables|Default|GetSpawn%20Height))) (Math|Conversions|ToVector(Float) (* (Variables|Default|GetRockSize) (Class|ProbabilityMethods|RayleighProbabilityNumber 1.0 0.5)))))
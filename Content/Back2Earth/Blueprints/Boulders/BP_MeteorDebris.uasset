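; BP_MeteorDebris is a sandstone boulder hazard that kills the player character on contact.
; The boulder's hit event casts to the third-person character and calls its Death function if it is still alive.
; A velocity check meant to spare players touching a stationary rock is left disconnected, so resting debris is also lethal.
; SetToDespawn gives the actor a long lifespan so it eventually removes itself, though nothing here calls it.
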(event OnComponentHit(SandstoneBoulder)
  (params (HitComponent :type Primitive%20Component%20Object%20Reference) (OtherActor :type Actor%20Object%20Reference) (OtherComp :type Primitive%20Component%20Object%20Reference) (NormalImpulse :type Vector :default "0, 0, 0") (Hit :type Hit%20Result%20Structure%20%28by%20ref%29))
  (bind _asbp_b2e_third_person_character (Utilities|Casting|CastToBP_B2E_ThirdPersonCharacter OtherActor))
  (if (Variables|/Game/Back2Earth/Blueprints/BP_B2E_ThirdPersonCharacter.BP_B2E_ThirdPersonCharacter_C|GetIsAlive _asbp_b2e_third_person_character)
    (Default|Death _asbp_b2e_third_person_character 3.0)))

(fn ConstructionScript)

(fn SettoDespawn
  (Actor|SetLifeSpan 3e+02))
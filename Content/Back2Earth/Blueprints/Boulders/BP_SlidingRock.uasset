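; BP_SlidingRock is a short-lived physics boulder hazard that kills the third-person player character on contact.
; A looping timer repeatedly applies a downward velocity impulse to the sandstone mesh and adds Y-axis torque whenever its spin about that axis is too slow.
; Component hits cast to BP_B2E_ThirdPersonCharacter and call its Death function, while a lifespan set on BeginPlay removes the rock automatically.
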(event OnComponentHit(SandstoneBoulder)
  (params (HitComponent :type Primitive%20Component%20Object%20Reference) (OtherActor :type Actor%20Object%20Reference) (OtherComp :type Primitive%20Component%20Object%20Reference) (NormalImpulse :type Vector :default "0, 0, 0") (Hit :type Hit%20Result%20Structure%20%28by%20ref%29))
  (bind _asbp_b2e_third_person_character (Utilities|Casting|CastToBP_B2E_ThirdPersonCharacter OtherActor))
  (Default|Death _asbp_b2e_third_person_character 3.0))

(event Custom|Update
  (bind _sandstone_boulder (Variables|Default|GetSandstone%20Boulder))
  (Physics|AddImpulse _sandstone_boulder "0.000000, 0,-300.000000" "None" true)
  (if (> 1e+02 (Math|Float|Absolute(Float) (.y (Physics|GetPhysicsAngularVelocityinDegrees _sandstone_boulder "None"))))
    (Class|PrimitiveComponent|AddTorqueinDegrees (Variables|Default|GetSandstone%20Boulder) "0,500.000000, 0" "None" false)))

(event EventBeginPlay
  (Actor|SetLifeSpan 25.0)
  (Utilities|Time|SetTimerbyEvent (delegate Custom|Update) 0.2 true))

(fn ConstructionScript)
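; Game mode for Back2Earth that applies per-level movement tuning to the third-person character and handles death and respawn.
; SetPlayerStuff caches speed, jump, gravity and acceleration values, which are reapplied after each respawn.
; OnKilled spawns and possesses a new character at SpawnTransform, or restarts the game if it is unset.
; On the Moon, respawn clears meteor debris and resets a timer-driven countdown shown in WBP_MoonInterface.
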(event Custom|CreateCountdown
  (bind _returnvalue (UserInterface|CreateWidget "/Game/Back2Earth/Blueprints/WBP_MoonInterface.WBP_MoonInterface_C"))
  (bind _output_get (Variables|Default|SetUIRef _returnvalue))
  (UserInterface|Viewport|AddtoViewport _output_get 0)
  (Utilities|Time|SetTimerbyEvent (delegate Custom|UpdateTimer) 0.01 true))

(event Custom|SetPlayerStuff
  (params (GModeWalkVelocity :type Float%20%28double-precision%29) (GModeZJumpMultiplier :type Float%20%28double-precision%29) (GModeAcceleration :type Float%20%28double-precision%29) (GModeRunVelocity :type Float%20%28double-precision%29) (PlayerGravityScale :type Float%20%28double-precision%29) (PlayerJumpZVelocity :type Float%20%28double-precision%29) (PlayerWalkSpeed :type Float%20%28double-precision%29) (PlayerRunMultiplier :type Float%20%28double-precision%29))
  (Variables|Default|SetCurrentLevelGModeWalkVelocity GModeWalkVelocity)
  (Variables|Default|SetCurrentLevelGModeZJumpMultiplier GModeZJumpMultiplier)
  (Variables|Default|SetCurrentLevelGModeAcceleration GModeAcceleration)
  (Variables|Default|SetCurrentLevelGModeRunVelocity GModeRunVelocity)
  (Variables|Default|SetCurrentLevelPlayerGravityScale PlayerGravityScale)
  (Variables|Default|SetCurrentLevelPlayerJumpZVelocity PlayerJumpZVelocity)
  (Variables|Default|SetCurrentLevelPlayerWalkSpeed PlayerWalkSpeed)
  (Variables|Default|SetCurrentLevelPlayerRunMultiplier PlayerRunMultiplier)
  (CallFunction|SetCharacterStuff))

(event Custom|Respawn
  (CallFunction|SetCharacterStuff)
  (bind _asbp_b2e_third_person_character (Utilities|Casting|CastToBP_B2E_ThirdPersonCharacter (Game|GetPlayerCharacter 0)))
  (Game|BindEventtoOnDestroyed _asbp_b2e_third_person_character (delegate Custom|On%20Killed))
  (bind _returnvalue (Game|GetCurrentLevelName true))
  (if (Utilities|Enum|Equal(Enum) _returnvalue "Moon")
    (bind _outactors (Actor|GetAllActorsOfClass "/Game/Back2Earth/Blueprints/Boulders/BP_MeteorDebris.BP_MeteorDebris_C"))
    (Actor|DestroyActor _outactors)
    (Variables|Default|SetCountdownWorking false)
    (Variables|Default|SetMoonTimeLeft (Variables|Default|GetMoonDefaultTimerTime))))

(event Custom|On%20Killed
  (params (DestroyedActor :type Actor%20Object%20Reference))
  (if (not (== (Math|Transform|MakeTransform "0, 0, 0") (Variables|Default|GetSpawn%20Transform)))
    (bind _returnvalue (Game|SpawnActorfromClass "/Game/Back2Earth/Blueprints/BP_B2E_ThirdPersonCharacter.BP_B2E_ThirdPersonCharacter_C" (Variables|Default|GetSpawn%20Transform) "AdjustIfPossibleButAlwaysSpawn" 0 0))
    (Pawn|Possess (Game|GetPlayerController 0) _returnvalue)
    (bind _asbp_b2e_third_person_character (Utilities|Casting|CastToBP_B2E_ThirdPersonCharacter (Game|Player|GetPlayerPawn 0)))
    (Physics|AddImpulse (Variables|/Script/Engine.Character|GetCharacterMovement _asbp_b2e_third_person_character) "0, 0,-1000.000000" true)
    (CallFunction|Respawn)
    (else
      (Class|GameMode|RestartGame))))

(event Custom|UpdateTimer
  (if (Variables|Default|GetCountdownWorking)
    (if (not (<= (Variables|Default|GetMoonTimeLeft) 0.0))
      (bind _output_get (Variables|Default|SetMoonTimeLeft (- (Variables|Default|GetMoonTimeLeft) 0.01)))
      (Default|SetTimeLeft (Variables|Default|GetUIRef) _output_get))
    (else
      (Default|SetTimeLeft (Variables|Default|GetUIRef) (Variables|Default|GetMoonTimeLeft)))))

(event EventBeginPlay
  (bind _asbp_b2e_third_person_character (Utilities|Casting|CastToBP_B2E_ThirdPersonCharacter (Game|GetPlayerCharacter 0)))
  (Game|BindEventtoOnDestroyed _asbp_b2e_third_person_character (delegate Custom|On%20Killed))
  (bind _returnvalue (Game|GetCurrentLevelName true))
  (if (Utilities|Enum|Equal(Enum) _returnvalue "Moon")
    (bind _outactors (Actor|GetAllActorsOfClass "/Game/Back2Earth/Blueprints/Boulders/BP_MeteorDebris.BP_MeteorDebris_C"))
    (Actor|DestroyActor _outactors)
    (Variables|Default|SetCountdownWorking false)
    (Variables|Default|SetMoonTimeLeft (Variables|Default|GetMoonDefaultTimerTime))))

(fn ConstructionScript)

(fn SetCharacterStuff
  (bind _asbp_b2e_third_person_character (Utilities|Casting|CastToBP_B2E_ThirdPersonCharacter (Game|GetPlayerCharacter 0)))
  (Variables|/Game/Back2Earth/Blueprints/BP_B2E_ThirdPersonCharacter.BP_B2E_ThirdPersonCharacter_C|SetGModeWalkVelocity _asbp_b2e_third_person_character (Variables|Default|GetCurrentLevelGModeWalkVelocity))
  (Variables|/Game/Back2Earth/Blueprints/BP_B2E_ThirdPersonCharacter.BP_B2E_ThirdPersonCharacter_C|SetGModeZJumpMultiplier _asbp_b2e_third_person_character (Variables|Default|GetCurrentLevelGModeZJumpMultiplier))
  (Variables|/Game/Back2Earth/Blueprints/BP_B2E_ThirdPersonCharacter.BP_B2E_ThirdPersonCharacter_C|SetGModeAcceleration _asbp_b2e_third_person_character (Variables|Default|GetCurrentLevelGModeAcceleration))
  (Variables|/Game/Back2Earth/Blueprints/BP_B2E_ThirdPersonCharacter.BP_B2E_ThirdPersonCharacter_C|SetGModeRunVelocity _asbp_b2e_third_person_character (Variables|Default|GetCurrentLevelGModeRunVelocity))
  (Variables|/Game/Back2Earth/Blueprints/BP_B2E_ThirdPersonCharacter.BP_B2E_ThirdPersonCharacter_C|SetRunMultiplier _asbp_b2e_third_person_character (Variables|Default|GetCurrentLevelPlayerRunMultiplier))
  (bind _output_get (Variables|/Game/Back2Earth/Blueprints/BP_B2E_ThirdPersonCharacter.BP_B2E_ThirdPersonCharacter_C|SetDefaultSpeed _asbp_b2e_third_person_character (Variables|Default|GetCurrentLevelPlayerWalkSpeed)))
  (Variables|/Script/Engine.CharacterMovementComponent|SetMaxWalkSpeed (Variables|/Script/Engine.Character|GetCharacterMovement _asbp_b2e_third_person_character) _output_get)
  (Variables|/Script/Engine.CharacterMovementComponent|SetGravityScale (Variables|/Script/Engine.Character|GetCharacterMovement _asbp_b2e_third_person_character) (Variables|Default|GetCurrentLevelPlayerGravityScale))
  (Variables|/Script/Engine.CharacterMovementComponent|SetJumpZVelocity (Variables|/Script/Engine.Character|GetCharacterMovement _asbp_b2e_third_person_character) (Variables|Default|GetCurrentLevelPlayerJumpZVelocity)))
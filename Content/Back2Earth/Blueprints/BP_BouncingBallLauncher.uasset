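; BP_BouncingBallLauncher is a launcher actor that repeatedly spawns BP_BouncingBall actors once Activate is called.
; Each spawn follows a random delay drawn from an exponential probability function using a minimum and exponential interval.
; Balls appear at SpawnLocationCube, oriented along the Arrow with uniform random pitch and yaw spread.
; The loop repeats while IsActive is true, and Deactivate clears that flag.
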(event Custom|Activate
  (bind _spreadz (Variables|Default|GetspreadZ))
  (bind _arrow (Variables|Default|GetArrow))
  (bind _spready (Variables|Default|GetspreadY))
  (bind _returnvalue (Transformation|GetWorldRotation _arrow))
  (Utilities|FlowControl|Delay (Class|ProbabilityMethods|ExponentialProbabilityNumber (Variables|Default|Getminimum_spawn_interval) (Variables|Default|Getexponential_spawn_interval)) :!label _label)
  (Game|SpawnActorfromClass "/Game/Back2Earth/Blueprints/BP_BouncingBall.BP_BouncingBall_C" (Math|Transform|MakeTransform (Transformation|GetWorldLocation (Variables|Default|GetSpawnLocationCube)) (Math|Rotator|MakeRotator (.roll _returnvalue) (+ (.pitch _returnvalue) (/ _spready -2.0) (Class|ProbabilityMethods|UniformProbabilityNumber 0.0 _spready)) (+ (.yaw _returnvalue) (/ _spreadz -2.0) (Class|ProbabilityMethods|UniformProbabilityNumber 0.0 _spreadz))) "1.000000,1.000000,1.000000") "Undefined" 0 0)
  (if (Variables|Default|GetisActive)
    (goto _label)))

(event EventBeginPlay)

(fn ConstructionScript)

(fn Deactivate
  (Variables|Default|SetisActive false))
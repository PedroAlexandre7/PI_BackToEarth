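; BP_MissileLauncher is an actor that automatically fires volleys of BP_Missile on a repeating timer from BeginPlay.
; Each cycle waits FireInterval, draws the missile count from a binomial distribution between min and max, and plays a launch sound if any fired.
; RandomSpread selects uniformly random or evenly spaced yaw offsets across a Spread cone centred on MissileSpawnArrow, with lone distributed missiles going straight along the arrow.
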(event EventBeginPlay
  (Utilities|FlowControl|Delay (Variables|Default|Getfire_interval) :!label _label)
  (Variables|Default|Setcurrent_number_projectiles (Class|ProbabilityMethods|BinomialProbabilityNumberMinMax (Variables|Default|Getmin_projectiles) (Variables|Default|Getmax_projectiles) (Variables|Default|Getbinomial_probability)))
  (if (Variables|Default|Getrandom_spread)
    (CallFunction|SpawnProjectileConeRandomSpread)
    (else
      (CallFunction|SpawnProjectileConeDistributedSpread)))
  (Math|Integer|CompareInt (Variables|Default|Getcurrent_number_projectiles)
    (:>
      (Audio|SpawnSoundatLocation "/Game/StarterContent/Audio/Explosion01.Explosion01" (Transformation|GetWorldLocation (Variables|Default|GetDefaultSceneRoot)) "0, 0, 0" 0.3 2.0 0.0 "/Game/Back2Earth/Sounds/MissileSoundAttenuation.MissileSoundAttenuation" 0)
      (goto _label))
    (:==
      (goto _label))))

(fn ConstructionScript)

(fn SpawnProjectileConeDistributedSpread
  (bind _current_number_projectiles (Variables|Default|Getcurrent_number_projectiles))
  (bind _spread (Variables|Default|Getspread))
  (bind _missilespawnarrow (Variables|Default|GetMissileSpawnArrow))
  (bind _returnvalue (Transformation|GetWorldTransform _missilespawnarrow))
  (bind _returnvalue_2 (- _current_number_projectiles 1))
  (Math|Integer|CompareInt _current_number_projectiles 1
    (:>
      (for _index (range 0 _returnvalue_2) :!label _label
        (Game|SpawnActorfromClass "/Game/Back2Earth/Blueprints/BP_Missile.BP_Missile_C" (Math|Transform|MakeTransform (.location _returnvalue) (Math|Rotator|MakeRotator (.roll (.rotation _returnvalue)) (.pitch (.rotation _returnvalue)) (+ (.yaw (.rotation _returnvalue)) (/ _spread -2.0) (* _index (/ _spread (Math|Conversions|ToFloat(Integer) _returnvalue_2))))) "1.000000,1.000000,1.000000") "AlwaysSpawn" 0 0)))
    (:==
      (Game|SpawnActorfromClass "/Game/Back2Earth/Blueprints/BP_Missile.BP_Missile_C" (Transformation|GetWorldTransform _missilespawnarrow) "AlwaysSpawn" 0 0))
    (:<
      (goto _label))))

(fn SpawnProjectileConeRandomSpread
  (bind _missilespawnarrow (Variables|Default|GetMissileSpawnArrow))
  (bind _spread (Variables|Default|Getspread))
  (bind _returnvalue (Transformation|GetWorldTransform _missilespawnarrow))
  (for _index (range 0 (- (Variables|Default|Getcurrent_number_projectiles) 1))
    (Game|SpawnActorfromClass "/Game/Back2Earth/Blueprints/BP_Missile.BP_Missile_C" (Math|Transform|MakeTransform (.location _returnvalue) (Math|Rotator|MakeRotator (.roll (.rotation _returnvalue)) (.pitch (.rotation _returnvalue)) (+ (.yaw (.rotation _returnvalue)) (/ _spread -2.0) (Class|ProbabilityMethods|UniformProbabilityNumber 0.0 _spread))) "1.000000,1.000000,1.000000") "AlwaysSpawn" 0 0)))